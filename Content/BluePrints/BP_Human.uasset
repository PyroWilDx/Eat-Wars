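; BP_Human is an AI-driven human character that seeks out the closest food until it dies.
; A loop started on BeginPlay re-targets the nearest food every fraction of a second with SimpleMoveToActor, then stops movement immediately and ends once the human is dead.
; Each tick, its health bar component rotates to face the player along the look-at direction from the human's location.
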(event `self.ReceiveBeginPlay`
  (bind _returnvalue (`self.GetIsDead` :!label _label))
  (if _returnvalue
    (`MovementComponent.StopMovementImmediately` (`self.CharacterMovement`))
    (else
      (bind _returnvalue_2 (`self.GetClosestFood` self))
      (if (`KismetSystemLibrary.IsValid` _returnvalue_2)
        (`AIBlueprintHelperLibrary.SimpleMoveToActor` (`AIBlueprintHelperLibrary.GetAIController` self) _returnvalue_2))
      (`KismetSystemLibrary.Delay` 0.2)
      (goto _label))))

(event `self.ReceiveTick`
  (params (DeltaSeconds :type "Float (single-precision)"))
  (bind _returnvalue (`self.GetPlayer` self))
  (if (`KismetSystemLibrary.IsValid` _returnvalue)
    (`SceneComponent.K2_SetWorldRotation` (`self.HealthBarComponent`) (`KismetMathLibrary.FindLookAtRotation` (`self.K2_GetActorLocation` self) (`self.K2_GetActorLocation` _returnvalue)) false false)))

(fn `UserConstructionScript`)