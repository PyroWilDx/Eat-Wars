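; BP_FoodPlayer is the player Blueprint that handles the game-over screen when the player dies.
; It polls the death state every Tick, using the game's paused state as a guard so the sequence runs only while unpaused.
; On death it pauses the game, creates WBP_Menu, fills in hit, killed-human and total damage stats from getter functions, then shows the menu and mouse cursor.
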(event `self.ReceiveTick`
  (params (DeltaSeconds :type "Float (single-precision)"))
  (bind _returnvalue (`self.GetIsDead`))
  (if (and _returnvalue (not (`GameplayStatics.IsGamePaused`)))
    (`GameplayStatics.SetGamePaused` true)
    (bind _returnvalue_2 (`|CreateWidget` "/Game/Blueprints/WBP_Menu.WBP_Menu_C"))
    (bind _returnvalue_3 (`self.GetHitNumberString`))
    (`TextBlock.SetText` (`/Game/Blueprints/WBP_Menu.Text_HitNumber` _returnvalue_2) (`KismetTextLibrary.Conv_StringToText` _returnvalue_3))
    (bind _returnvalue_4 (`self.GetKilledHumanCountString`))
    (`TextBlock.SetText` (`/Game/Blueprints/WBP_Menu.Text_KilledHumanCount` _returnvalue_2) (`KismetTextLibrary.Conv_StringToText` _returnvalue_4))
    (bind _returnvalue_5 (`self.GetTotalDamageString`))
    (`TextBlock.SetText` (`/Game/Blueprints/WBP_Menu.Text_TotalDamage` _returnvalue_2) (`KismetTextLibrary.Conv_StringToText` _returnvalue_5))
    (`UserWidget.AddToViewport` _returnvalue_2 0)
    (set `PlayerController.bShowMouseCursor` true (`GameplayStatics.GetPlayerController` 0))))

(fn `UserConstructionScript`)